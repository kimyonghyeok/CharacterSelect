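; BP_GM_Menu is the menu game mode, which restores the saved character's look on the main menu character at BeginPlay.
; If a save exists in Slot_01 and holds a non-empty player name, it passes the stored third-person mesh, materials and animation class to BP_MainMenuCharacter's UpdateCharacter.
; If no save exists, it creates a BP_SaveGame and writes it to that slot.
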(event `self.ReceiveBeginPlay`
  (bind _returnvalue (`GameplayStatics.DoesSaveGameExist` "Slot_01"))
  (if _returnvalue
    (bind _returnvalue_2 (`GameplayStatics.LoadGameFromSlot` "Slot_01"))
    (bind _asbp_save_game (cast `/Game/SimpleCharacterSelect/Blueprints/BP_SaveGame` _returnvalue_2))
    (bind _returnvalue_3 (`GameplayStatics.GetActorOfClass` "/Game/SimpleCharacterSelect/Blueprints/BP_MainMenuCharacter.BP_MainMenuCharacter_C"))
    (`/Engine/EditorBlueprintResources/StandardMacros.IsValid` _returnvalue_3
      (:`Is Valid`
        (bind (_playerdetails_name _playerdetails_description _playerdetails_locked _playerdetails_portrait _playerdetails_thirdperson_mesh _playerdetails_firstperson_mesh _playerdetails_materials _playerdetails_pose _playerdetails_skins _playerdetails_animclass) (break `/Game/SimpleCharacterSelect/Blueprints/S_CharacterSelect` (`/Game/SimpleCharacterSelect/Blueprints/BP_SaveGame.PlayerDetails` _asbp_save_game)))
        (if (not (`KismetTextLibrary.TextIsEmpty` _playerdetails_name))
          (`/Game/SimpleCharacterSelect/Blueprints/BP_MainMenuCharacter.UpdateCharacter` _returnvalue_3 _playerdetails_thirdperson_mesh _playerdetails_materials _playerdetails_animclass))))
    (else
      (bind _returnvalue_4 (`GameplayStatics.CreateSaveGameObject` "/Game/SimpleCharacterSelect/Blueprints/BP_SaveGame.BP_SaveGame_C"))
      (bind _output_get (set `self.SaveGame` _returnvalue_4))
      (`GameplayStatics.SaveGameToSlot` _output_get "Slot_01"))))

(fn `UserConstructionScript`)